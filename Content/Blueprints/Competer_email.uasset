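; Computer email interactable actor that shows a WBP_ReadNotes widget when O is pressed inside its box trigger.
; Box overlap sets a can-show flag, and both begin and end overlap enable input.
; Opening the widget hides the Plane and TextRender and sets look/move ignore to false.
; Later presses only remove the widget, since the nodes resetting the visible flag and setting ignore to true are unconnected.
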(event OnComponentBeginOverlap(Box)
  (params (OverlappedComponent :type Primitive%20Component%20Object%20Reference) (OtherActor :type Actor%20Object%20Reference) (OtherComp :type Primitive%20Component%20Object%20Reference) (OtherBodyIndex :type Integer) (bFromSweep :type Boolean) (SweepResult :type Hit%20Result%20Structure%20%28by%20ref%29))
  (Input|EnableInput (Game|GetPlayerController 0))
  (Variables|Default|SetcanShoWWBP true))

(event OnComponentEndOverlap(Box)
  (params (OverlappedComponent :type Primitive%20Component%20Object%20Reference) (OtherActor :type Actor%20Object%20Reference) (OtherComp :type Primitive%20Component%20Object%20Reference) (OtherBodyIndex :type Integer))
  (Input|EnableInput (Game|GetPlayerController 0))
  (Variables|Default|SetcanShoWWBP false))

(event Input|KeyboardEvents|O
  (params (Key :type Key%20Structure :default "None"))
  (bind _returnvalue (Game|GetPlayerController 0))
  (:Pressed
    (if (Variables|Default|GetcanShoWWBP)
      (if (Variables|Default|GetbIsWBPVisible)
        (Widget|RemovefromParent (stale _returnvalue_2))
        (else
          (bind _returnvalue_2 (Game|ConstructObjectfromClass "/Game/Blueprints/WBP_ReadNotes.WBP_ReadNotes_C"))
          (UserInterface|Viewport|AddtoViewport _returnvalue_2 0)
          (Input|SetIgnoreLookInput _returnvalue false)
          (Input|SetIgnoreMoveInput _returnvalue false)
          (Variables|Default|SetbIsWBPVisible true)
          (Rendering|SetVisibility (Variables|Default|GetPlane) false false)
          (Rendering|SetVisibility (Variables|Default|GetTextRender) false false))))))

(fn ConstructionScript)