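; BP_Duck_Game runs a duck tapping minigame that pays the player money for repeated Space presses.
; StartGame creates the WBP_Duck_Game widget, passes itself to it, enables the cursor with game-and-UI input, and activates the game.
; Each press scales the widget and advances a tap counter, with release unscaling it.
; At the TapsToMoney threshold it credits the character's BPCharacteristics, resets the count and briefly shows a notification.
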(event Custom|Start%20Game
  (bind _returnvalue (Game|GetPlayerController 0))
  (bind _returnvalue_2 (Game|ConstructObjectfromClass "/Game/Blueprints/UI/WBP_Duck_Game.WBP_Duck_Game_C"))
  (bind _output_get (Variables|Default|SetWidget _returnvalue_2))
  (UserInterface|Viewport|AddtoViewport _output_get 0)
  (Variables|/Game/Blueprints/UI/WBP_Duck_Game.WBP_Duck_Game_C|SetGame _output_get self)
  (Input|SetInputModeGameandUI _returnvalue (Variables|Default|GetWidget) "DoNotLock" true false)
  (Variables|/Script/Engine.PlayerController|SetbShowMouseCursor _returnvalue true)
  (Variables|Default|SetIsGameOn true))

(event Custom|Add%20One
  (bind _result (Math|Integer|IncrementInt (Variables|Default|GetTapsCount))
    (:%20%20
      (if (== _result (Variables|Default|GetTapsToMoney))
        (bind _returnvalue (Actor|GetActorOfClass "/Game/ThirdPerson/Blueprints/BP_ThirdPersonCharacter.BP_ThirdPersonCharacter_C"))
        (Default|AddMoney (Variables|/Game/ThirdPerson/Blueprints/BP_ThirdPersonCharacter.BP_ThirdPersonCharacter_C|GetBP_Characteristics _returnvalue) 1)
        (Variables|Default|SetTapsCount 0)
        (Variables|/Script/UMG.Widget|SetVisibility (Variables|/Game/Blueprints/UI/WBP_Duck_Game.WBP_Duck_Game_C|GetNotify (Variables|Default|GetWidget)) "Visible")
        (Utilities|Time|SetTimerbyEvent (delegate Custom|Hife%20Notify) 1.0)))))

(event Custom|Hife%20Notify
  (Variables|/Script/UMG.Widget|SetVisibility (Variables|/Game/Blueprints/UI/WBP_Duck_Game.WBP_Duck_Game_C|GetNotify (Variables|Default|GetWidget)) "Hidden"))

(event EventBeginPlay)

(event EventTick
  (params (DeltaSeconds :type Float%20%28single-precision%29)))

(event Input|KeyboardEvents|SpaceBar
  (params (Key :type Key%20Structure :default "None"))
  (bind _widget (Variables|Default|GetWidget))
  (:Pressed
    (if (Variables|Default|GetIsGameOn)
      (Default|Scale _widget)
      (CallFunction|AddOne)))
  (:Released
    (Default|Unscale _widget)))