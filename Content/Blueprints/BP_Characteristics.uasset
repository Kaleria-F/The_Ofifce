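; BP_Characteristics tracks a character's career stats (Charisma, Qualification, Productivity), Money and a job Level running from Intern to TeamLead.
; StartShow creates the WBP_StatsInfo widget, passes itself to it and caches the next level and its threshold via GetNextLevelInfo.
; Each stat Add event calls LevelUp, which recursively promotes while all three stats meet the threshold, stopping at TeamLead.
; AddMoney only changes Money.
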(event Custom|Level%20Up
  (if (Math|Boolean|ANDBoolean (>= (Variables|Default|GetCharisma) (Variables|Default|GetNextStateValue)) (>= (Variables|Default|GetQualification) (Variables|Default|GetNextStateValue)) (>= (Variables|Default|GetProductivity) (Variables|Default|GetNextStateValue)) (Utilities|Enum|NotEqual(Enum) (Variables|Default|GetLevel) "NewEnumerator5"))
    (Variables|Default|SetLevel (Variables|Default|GetNextLevel))
    (bind (_next_level _minstatsvalue) (CallFunction|GetNextLevelInfo))
    (Variables|Default|SetNextLevel _next_level)
    (Variables|Default|SetNextStateValue _minstatsvalue)
    (CallFunction|LevelUp)))

(event Custom|Add%20Money
  (params (Money :type Integer))
  (Variables|Default|SetMoney (+ Money (Variables|Default|GetMoney))))

(event Custom|Add%20Charisma
  (params (Charisma :type Integer))
  (Variables|Default|SetCharisma (+ Charisma (Variables|Default|GetCharisma)))
  (CallFunction|LevelUp))

(event Custom|Add%20Productivity
  (params (Qualification :type Integer))
  (Variables|Default|SetProductivity (+ Qualification (Variables|Default|GetProductivity)))
  (CallFunction|LevelUp))

(event Custom|Add%20Qualification
  (params (Qualification :type Integer))
  (Variables|Default|SetQualification (+ Qualification (Variables|Default|GetQualification)))
  (CallFunction|LevelUp))

(event Custom|Start%20Show
  (bind _returnvalue (Game|ConstructObjectfromClass "/Game/Blueprints/WBP_StatsInfo.WBP_StatsInfo_C"))
  (bind _output_get (Variables|Default|SetStatsInfoUI _returnvalue))
  (UserInterface|Viewport|AddtoViewport _output_get 0)
  (Variables|/Game/Blueprints/WBP_StatsInfo.WBP_StatsInfo_C|SetStatsInfo _output_get self)
  (bind (_next_level _minstatsvalue) (CallFunction|GetNextLevelInfo))
  (Variables|Default|SetNextLevel _next_level)
  (Variables|Default|SetNextStateValue _minstatsvalue))

(event EventTick
  (params (DeltaSeconds :type Float%20%28single-precision%29)))

(fn GetNextLevelInfo
  (bind _level (Variables|Default|GetLevel))
  (bind _returnvalue (Utilities|Select :Index _level :NewEnumerator1 "NewEnumerator2" :NewEnumerator2 "NewEnumerator3" :NewEnumerator3 "NewEnumerator4" :NewEnumerator4 "NewEnumerator5" :NewEnumerator5 "NewEnumerator5"))
  (return _returnvalue (Utilities|Select :Index _returnvalue :NewEnumerator1 10 :NewEnumerator2 30 :NewEnumerator3 60 :NewEnumerator4 100 :NewEnumerator5 150)))