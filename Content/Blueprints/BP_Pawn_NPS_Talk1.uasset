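; BP_Pawn_NPS_Talk1 is a talk pawn that starts a dialogue view when the third-person character enters its InteractionZone.
; Overlap saves the follow camera's transform, snaps it to CameraTarget, blocks look and move input, and shows WBP_DialogWindow for 15 seconds.
; The logic restoring camera and input is disconnected, so both stay changed after the window closes.
; GetDialogueWidget separately exposes the DialogueWidgetComponent's widget, unused here.
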(event OnComponentBeginOverlap(InteractionZone)
  (params (OverlappedComponent :type Primitive%20Component%20Object%20Reference) (OtherActor :type Actor%20Object%20Reference) (OtherComp :type Primitive%20Component%20Object%20Reference) (OtherBodyIndex :type Integer) (bFromSweep :type Boolean) (SweepResult :type Hit%20Result%20Structure%20%28by%20ref%29))
  (bind _returnvalue (Game|GetPlayerController 0))
  (bind _cameratarget (Variables|Default|GetCameraTarget))
  (bind _asbp_third_person_character (Utilities|Casting|CastToBP_ThirdPersonCharacter OtherActor))
  (Variables|Default|SetInitialCameraPosition%20 (Transformation|GetWorldLocation (Variables|/Game/ThirdPerson/Blueprints/BP_ThirdPersonCharacter.BP_ThirdPersonCharacter_C|GetFollowCamera _asbp_third_person_character)))
  (Variables|Default|SetInitialCamerRotation (Math|Rotator|GetRotationXVector (Transformation|GetWorldRotation (Variables|/Game/ThirdPerson/Blueprints/BP_ThirdPersonCharacter.BP_ThirdPersonCharacter_C|GetFollowCamera _asbp_third_person_character))))
  (Transformation|SetWorldLocationAndRotation (Variables|/Game/ThirdPerson/Blueprints/BP_ThirdPersonCharacter.BP_ThirdPersonCharacter_C|GetFollowCamera _asbp_third_person_character) (Transformation|GetWorldLocation _cameratarget) (Transformation|GetWorldRotation _cameratarget) false false)
  (Input|SetIgnoreLookInput _returnvalue true)
  (Input|SetIgnoreMoveInput _returnvalue true)
  (bind _returnvalue_2 (UserInterface|CreateWidget "/Game/Blueprints/WBP_DialogWindow.WBP_DialogWindow_C"))
  (UserInterface|Viewport|AddtoViewport _returnvalue_2 0)
  (Utilities|FlowControl|Delay 15.0)
  (Widget|RemovefromParent _returnvalue_2))

(event OnComponentEndOverlap(InteractionZone)
  (params (OverlappedComponent :type Primitive%20Component%20Object%20Reference) (OtherActor :type Actor%20Object%20Reference) (OtherComp :type Primitive%20Component%20Object%20Reference) (OtherBodyIndex :type Integer))
  (Utilities|Casting|CastToBP_ThirdPersonCharacter OtherActor))

(event EventBeginPlay)

(event Collision|EventActorBeginOverlap
  (params (OtherActor :type Actor%20Object%20Reference)))

(event EventTick
  (params (DeltaSeconds :type Float%20%28single-precision%29)))

(fn ConstructionScript)

(fn GetDialogueWidget
  (bind _aswbp_dialog_window (Utilities|Casting|CastToWBP_DialogWindow (UserInterface|GetUserWidgetObject (Variables|Default|GetDialogueWidgetComponent))))
  (return _aswbp_dialog_window))