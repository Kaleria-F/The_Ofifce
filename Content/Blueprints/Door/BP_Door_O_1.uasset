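; BP_Door_O_1 is a door that the player swings open and closed by pressing O while input is enabled.
; Three trigger boxes toggle player 0's input on overlap without checking the overlapping actor, and two also show or hide their own prompt text.
; Timeline_Door drives door yaw forward or in reverse, with DoorTime blocking presses mid-swing.
; DoorOpen picks the direction and is true when yaw is zero or below.
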(event OnComponentBeginOverlap(Box)
  (params (OverlappedComponent :type Primitive%20Component%20Object%20Reference) (OtherActor :type Actor%20Object%20Reference) (OtherComp :type Primitive%20Component%20Object%20Reference) (OtherBodyIndex :type Integer) (bFromSweep :type Boolean) (SweepResult :type Hit%20Result%20Structure%20%28by%20ref%29))
  (Input|EnableInput (Game|GetPlayerController 0)))

(event OnComponentEndOverlap(Box)
  (params (OverlappedComponent :type Primitive%20Component%20Object%20Reference) (OtherActor :type Actor%20Object%20Reference) (OtherComp :type Primitive%20Component%20Object%20Reference) (OtherBodyIndex :type Integer))
  (Input|DisableInput (Game|GetPlayerController 0)))

(event OnComponentBeginOverlap(Box1)
  (params (OverlappedComponent :type Primitive%20Component%20Object%20Reference) (OtherActor :type Actor%20Object%20Reference) (OtherComp :type Primitive%20Component%20Object%20Reference) (OtherBodyIndex :type Integer) (bFromSweep :type Boolean) (SweepResult :type Hit%20Result%20Structure%20%28by%20ref%29))
  (Input|EnableInput (Game|GetPlayerController 0))
  (Rendering|SetVisibility (Variables|Default|GetText1) true false))

(event OnComponentEndOverlap(Box1)
  (params (OverlappedComponent :type Primitive%20Component%20Object%20Reference) (OtherActor :type Actor%20Object%20Reference) (OtherComp :type Primitive%20Component%20Object%20Reference) (OtherBodyIndex :type Integer))
  (Input|DisableInput (Game|GetPlayerController 0))
  (Rendering|SetVisibility (Variables|Default|GetText1) false false))

(event OnComponentBeginOverlap(Box2)
  (params (OverlappedComponent :type Primitive%20Component%20Object%20Reference) (OtherActor :type Actor%20Object%20Reference) (OtherComp :type Primitive%20Component%20Object%20Reference) (OtherBodyIndex :type Integer) (bFromSweep :type Boolean) (SweepResult :type Hit%20Result%20Structure%20%28by%20ref%29))
  (Input|EnableInput (Game|GetPlayerController 0))
  (Rendering|SetVisibility (Variables|Default|GetText2) true false))

(event OnComponentEndOverlap(Box2)
  (params (OverlappedComponent :type Primitive%20Component%20Object%20Reference) (OtherActor :type Actor%20Object%20Reference) (OtherComp :type Primitive%20Component%20Object%20Reference) (OtherBodyIndex :type Integer))
  (Input|DisableInput (Game|GetPlayerController 0))
  (Rendering|SetVisibility (Variables|Default|GetText2) false false))

(event EventBeginPlay)

(event Collision|EventActorBeginOverlap
  (params (OtherActor :type Actor%20Object%20Reference)))

(event EventTick
  (params (DeltaSeconds :type Float%20%28single-precision%29)))

(event Input|KeyboardEvents|O
  (params (Key :type Key%20Structure))
  (:Pressed
    (if (Variables|Default|GetDoorTime)
      (if (Variables|Default|GetDoorOpen)
        (Variables|Default|SetDoorTime false)
        (bind _новая_дорожка_0 (Timeline|Timeline_Door Play)
          (:Update
            (Transformation|SetRelativeRotation (Variables|Default|GetDoor) (Math|Rotator|MakeRotator 0.0 0.0 _новая_дорожка_0) false false)
            (Variables|Default|SetDoorOpen (not (> _новая_дорожка_0 0.0))))
          (:Finished
            (Variables|Default|SetDoorTime true)))
        (else
          (Variables|Default|SetDoorTime false)
          (Timeline|Timeline_Door ReverseFromEnd))))))

(fn ConstructionScript)