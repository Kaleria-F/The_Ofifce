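; BP_ToTouch is a collectible actor that the third-person character picks up by touching it.
; When Sphere1 begins overlapping a BP_ThirdPersonCharacter, it checks that the character's PersonLevel is the first enum value (NewEnumerator0).
; If so, it destroys itself, increments the character's NumberTouches, and pushes that count to the character's WidgetTouch to refresh its text.
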(event OnComponentBeginOverlap(Sphere1)
  (params (OverlappedComponent :type Primitive%20Component%20Object%20Reference) (OtherActor :type Actor%20Object%20Reference) (OtherComp :type Primitive%20Component%20Object%20Reference) (OtherBodyIndex :type Integer) (bFromSweep :type Boolean) (SweepResult :type Hit%20Result%20Structure%20%28by%20ref%29))
  (bind _asbp_third_person_character (Utilities|Casting|CastToBP_ThirdPersonCharacter OtherActor))
  (if (Utilities|Enum|Equal(Enum) (Variables|/Game/ThirdPerson/Blueprints/BP_ThirdPersonCharacter.BP_ThirdPersonCharacter_C|GetPersonLevel _asbp_third_person_character) "NewEnumerator0")
    (Actor|DestroyActor)
    (bind _output_get (Variables|/Game/ThirdPerson/Blueprints/BP_ThirdPersonCharacter.BP_ThirdPersonCharacter_C|SetNumberTouches _asbp_third_person_character (+ (Variables|/Game/ThirdPerson/Blueprints/BP_ThirdPersonCharacter.BP_ThirdPersonCharacter_C|GetNumberTouches _asbp_third_person_character) 1)))
    (Variables|/Game/Blueprints/WBP_NumberTouches.WBP_NumberTouches_C|SetCollectedCount (Variables|/Game/ThirdPerson/Blueprints/BP_ThirdPersonCharacter.BP_ThirdPersonCharacter_C|GetwidgetTouch _asbp_third_person_character) _output_get)
    (Default|UpdateText (Variables|/Game/ThirdPerson/Blueprints/BP_ThirdPersonCharacter.BP_ThirdPersonCharacter_C|GetwidgetTouch _asbp_third_person_character))))

(event EventBeginPlay)

(event Collision|EventActorBeginOverlap
  (params (OtherActor :type Actor%20Object%20Reference)))

(event EventTick
  (params (DeltaSeconds :type Float%20%28single-precision%29)))

(fn ConstructionScript)