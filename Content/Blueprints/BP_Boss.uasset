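; Boss enemy that patrols waypoints and can catch the player, sending them back to a stored location.
; Pressing E starts a looping AIMoveTo patrol, whose wrap check skips the last point.
; CheckForPlayer tests distance, facing cone and line trace, then resets the player, but nothing here calls it.
; Its try-again widget is removed immediately, as the delayed Delete timer only prints.
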(event Custom|PatrolToNextPoint
  (if (Variables|Default|GetIsPatrolling)
    (AI|AIMoveTo self "0, 0, 0" (Utilities|Array|Get(acopy) (Variables|Default|GetPatrolPoints) (Variables|Default|GetCurrentPatrolIndex)) 5e+01 false
      (:OnSuccess
        (Variables|Default|SetCurrentPatrolIndex (+ (Variables|Default|GetCurrentPatrolIndex) 1))
        (if (>= (+ (Variables|Default|GetCurrentPatrolIndex) 1) (Utilities|Array|Length (Variables|Default|GetPatrolPoints)))
          (Variables|Default|SetCurrentPatrolIndex 0)
          (Development|PrintString "Hello")
          (CallFunction|PatroltoNextPoint)
          (else
            (CallFunction|PatroltoNextPoint)))))))

(event EventBeginPlay)

(event Collision|EventActorBeginOverlap
  (params (OtherActor :type Actor%20Object%20Reference)))

(event EventTick
  (params (DeltaSeconds :type Float%20%28single-precision%29)))

(event Input|KeyboardEvents|E
  (params (Key :type Key%20Structure))
  (:Pressed
    (Variables|Default|SetIsPatrolling true)
    (CallFunction|PatroltoNextPoint)))

(fn ConstructionScript)

(fn CheckforPlayer
  (bind _returnvalue (Game|GetPlayerCharacter 0))
  (bind _returnvalue_2 (Transformation|GetActorLocation))
  (bind _returnvalue_3 (Transformation|GetActorLocation _returnvalue))
  (bind _returnvalue_4 (- _returnvalue_3 _returnvalue_2))
  (if (not (> (Math|Vector|VectorLength _returnvalue_4) 5e+02))
    (if (not (< (Math|Vector|DotProduct (Math|Vector|Normalize _returnvalue_4) (Transformation|GetActorForwardVector)) 0.7))
      (bind _outhit (Collision|LineTraceByChannel _returnvalue_2 _returnvalue_3 "TraceTypeQuery1" false 0 "ForDuration"))
      (if (.bBlockingHit (Collision|BreakHitResult _outhit))
        (bind _asbp_third_person_character (Utilities|Casting|CastToBP_ThirdPersonCharacter (Components|GetOwner (.HitComponent (Collision|BreakHitResult _outhit))))
          (:then
            (if (Utilities|IsValid _asbp_third_person_character)
              (Variables|/Game/ThirdPerson/Blueprints/BP_ThirdPersonCharacter.BP_ThirdPersonCharacter_C|SetIsFound _asbp_third_person_character true)
              (Transformation|SetActorLocation _asbp_third_person_character (Variables|Default|GetStLoc) false false)
              (Variables|/Game/ThirdPerson/Blueprints/BP_ThirdPersonCharacter.BP_ThirdPersonCharacter_C|SetIsFound _asbp_third_person_character false)
              (bind _returnvalue_5 (UserInterface|CreateWidget "/Game/Blueprints/WBP_Tryagain.WBP_Tryagain_C"))
              (UserInterface|Viewport|AddtoViewport _returnvalue_5 0)
              (Utilities|Time|SetTimerbyFunctionName 0 "Delete" 3.0)
              (Widget|RemovefromParent _returnvalue_5)
              (CallFunction|PatroltoNextPoint)))
          (:CastFailed
            (Development|PrintString "Hello")))))))

(fn Delete
  (Development|PrintString "Hello"))