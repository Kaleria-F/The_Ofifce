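; BP_CharacteristicSphere is a test pickup sphere that boosts a BP_ThirdPersonCharacter's characteristics when that character overlaps it.
; Each overlap adds a random amount to Charisma, Productivity or Qualification in turn, then teleports the sphere to a random X/Y position at zero height.
; The rotation comes from FlipFlop3, a local macro that nests FlipFlops and loops back on the fourth state to make a three-way cycle.
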(event OnComponentBeginOverlap(Sphere1)
  (params (OverlappedComponent :type Primitive%20Component%20Object%20Reference) (OtherActor :type Actor%20Object%20Reference) (OtherComp :type Primitive%20Component%20Object%20Reference) (OtherBodyIndex :type Integer) (bFromSweep :type Boolean) (SweepResult :type Hit%20Result%20Structure%20%28by%20ref%29))
  (bind _returnvalue (Math|Random|RandomIntegerinRange 30 50))
  (bind _asbp_third_person_character (Utilities|Casting|CastToBP_ThirdPersonCharacter OtherActor))
  (Utilities|FlipFlop3
    (:A
      (Default|AddCharisma (Variables|/Game/ThirdPerson/Blueprints/BP_ThirdPersonCharacter.BP_ThirdPersonCharacter_C|GetBP_Characteristics _asbp_third_person_character) _returnvalue))
    (:B
      (Default|AddProductivity (Variables|/Game/ThirdPerson/Blueprints/BP_ThirdPersonCharacter.BP_ThirdPersonCharacter_C|GetBP_Characteristics _asbp_third_person_character) _returnvalue))
    (:C
      (Default|AddQualification (Variables|/Game/ThirdPerson/Blueprints/BP_ThirdPersonCharacter.BP_ThirdPersonCharacter_C|GetBP_Characteristics _asbp_third_person_character) _returnvalue)))
  (Transformation|Teleport (Math|Vector|MakeVector (Math|Conversions|ToFloat(Integer) (Math|Random|RandomIntegerinRange 500 1500)) (Math|Conversions|ToFloat(Integer) (Math|Random|RandomIntegerinRange 500 1500)) 0.0) "0, 0, 0"))

(event EventBeginPlay)

(event Collision|EventActorBeginOverlap
  (params (OtherActor :type Actor%20Object%20Reference)))

(event EventTick
  (params (DeltaSeconds :type Float%20%28single-precision%29)))

(fn ConstructionScript)